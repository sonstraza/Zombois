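; Zombie spawner actor that creates AI zombies of the InputZombie class at random points inside its SpawnVolume.
; BeginPlay copies ZombieInput to the first spawner found in the level, spawns one zombie immediately, and starts a looping SpawnZombie timer.
; That timer targets the first spawner's ZombieInput object rather than the spawner itself.
; Each SpawnZombie call gives the new pawn the BT_Zombie behavior tree.
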(event `self.ReceiveBeginPlay`
  (bind _outactors (`GameplayStatics.GetAllActorsOfClass` "BP_Actor_ZombieSpawner_C"))
  (bind _output_get (set `/Game/ZombiBois/Zombies/BP_Actor_ZombieSpawner.ZombieInput` (`self.ZombieInput`) (`|GetArrayItem` _outactors)))
  (`KismetSystemLibrary.K2_SetTimer` _output_get "SpawnZombie" 1.0 true)
  (`self.SpawnZombie`))

(event `self.ReceiveTick`
  (params (DeltaSeconds :type "Float (single-precision)")))

(event `SpawnZombie`
  (bind _spawnvolume (`self.SpawnVolume`))
  (`AIBlueprintHelperLibrary.SpawnAIFromClass` (`self.Input_Zombie`) "/Game/FPS_Game/Blueprints/Bonus/AI/Zombie/BT_Zombie.BT_Zombie" (`KismetMathLibrary.RandomPointInBoundingBox` (`SceneComponent.K2_GetComponentLocation` _spawnvolume) (`BoxComponent.GetScaledBoxExtent` _spawnvolume)) (struct) false null))

(fn `UserConstructionScript`)