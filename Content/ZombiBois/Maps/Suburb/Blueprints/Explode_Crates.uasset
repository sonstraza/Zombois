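; Suburb map Blueprint actor that launches six crate components with a physics impulse, sideways along +Y and upward, as soon as play begins.
; BeginPlay applies the same impulse to every crate in one AddImpulse call.
; The Trigger overlap event is empty, and leftover nodes for a CanExplode gate, a Player tag check and enabling physics simulation are disconnected, so the launch is unconditional.
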(event `self.ReceiveBeginPlay`
  (`PrimitiveComponent.AddImpulse` (`self.Crate_1`) (0.0 20000.0 20000.0) "None" false)
  (`PrimitiveComponent.AddImpulse` (`self.Crate_2`) (0.0 20000.0 20000.0) "None" false)
  (`PrimitiveComponent.AddImpulse` (`self.Crate_3`) (0.0 20000.0 20000.0) "None" false)
  (`PrimitiveComponent.AddImpulse` (`self.Crate_4`) (0.0 20000.0 20000.0) "None" false)
  (`PrimitiveComponent.AddImpulse` (`self.Crate_5`) (0.0 20000.0 20000.0) "None" false)
  (`PrimitiveComponent.AddImpulse` (`self.Crate_6`) (0.0 20000.0 20000.0) "None" false))

(event `self.Trigger.OnComponentBeginOverlap`
  (params (OverlappedComponent :type "PrimitiveComponent Object Reference") (OtherActor :type "Actor Object Reference") (OtherComp :type "PrimitiveComponent Object Reference") (OtherBodyIndex :type Integer) (bFromSweep :type Boolean) (SweepResult :type "HitResult Structure (by ref)")))

(fn `UserConstructionScript`)