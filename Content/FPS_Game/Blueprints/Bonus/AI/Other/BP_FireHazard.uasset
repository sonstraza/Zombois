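; BP_FireHazard is a fire hazard actor that plays a sound on spawn and deals small repeated damage to actors inside its sphere.
; Overlap events maintain an actor list and start a looping timer, which applies damage only to actors still overlapping the sphere.
; When extinguishable, it waits out its lifetime, deactivates particles, light, collision and the damage timer, then destroys itself after a short delay.
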(event `self.ReceiveBeginPlay`
  (`GameplayStatics.PlaySoundAtLocation` null (`self.K2_GetActorLocation`))
  (if (`self.Extinguishable`)
    (`KismetSystemLibrary.Delay` (`self.Lifetime`))
    (`ActorComponent.Deactivate` (`self.ParticleSystem`))
    (`ActorComponent.Deactivate` (`self.PointLight`))
    (`PrimitiveComponent.SetCollisionEnabled` (`self.Sphere`) "NoCollision")
    (`KismetSystemLibrary.K2_ClearTimer` null "Damage")
    (`KismetSystemLibrary.Delay` 2.0)
    (`self.K2_DestroyActor`)))

(event `self.ReceiveActorBeginOverlap`
  (params (OtherActor :type "Actor Object Reference"))
  (`KismetArrayLibrary.Array_Add` (`self.OverlapActors`) OtherActor)
  (`KismetSystemLibrary.K2_SetTimer` null "Damage" 0.5 true))

(event `self.ReceiveActorEndOverlap`
  (params (OtherActor :type "Actor Object Reference"))
  (`KismetArrayLibrary.Array_RemoveItem` (`self.OverlapActors`) OtherActor))

(event `Damage`
  (for _array_element (`self.OverlapActors`)
    (if (`PrimitiveComponent.IsOverlappingActor` (`self.Sphere`) _array_element)
      (`GameplayStatics.ApplyDamage` _array_element 0.1 null self))))

(fn `UserConstructionScript`)