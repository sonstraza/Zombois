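; BP_WayPoint is an objective waypoint marker whose Widget shows only while its assigned objective is the current one.
; On BeginPlay it caches the BP_GameModeObjectives game mode and starts a short looping timer.
; Each tick of that timer compares the game mode's CurrentObjectiveIndex with the waypoint's CurrentObjectiveActive and sets the Widget's visibility, polling rather than binding to objective changes.
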(event `self.ReceiveBeginPlay`
  (bind _asbp_game_mode_objectives (cast `/Game/FPS_Game/Blueprints/Bonus/Objectives/BP_GameModeObjectives` (`GameplayStatics.GetGameMode`)))
  (set `self.GameModeCast` _asbp_game_mode_objectives)
  (`KismetSystemLibrary.K2_SetTimer` null "WayPointVisibility" 0.2 true))

(event `WayPointVisibility`
  (bind _gamemodecast (`self.GameModeCast`))
  (`/Engine/EditorBlueprintResources/StandardMacros.IsValid` _gamemodecast
    (:`Is Valid`
      (`SceneComponent.SetVisibility` (`self.Widget`) (== (`/Game/FPS_Game/Blueprints/Bonus/Objectives/BP_GameModeObjectives.CurrentObjectiveIndex` _gamemodecast) (`self.CurrentObjectiveActive`)) false))))

(fn `UserConstructionScript`)