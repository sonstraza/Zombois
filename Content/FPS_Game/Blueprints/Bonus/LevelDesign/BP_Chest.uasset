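; Loot chest that the player opens through the interaction interface to get random weapons.
; Overlap with a BP_CharacterBase toggles the HUD interact prompt and a custom-depth highlight on the chest meshes.
; Interaction fires once, playing a sound and a timeline that rotates the lid open and disables the box collision.
; When the timeline finishes, it spawns one of eight random weapons at each of two sphere markers.
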(event `self.ReceiveActorBeginOverlap`
  (params (OtherActor :type "Actor Object Reference"))
  (bind _asbp_character_base (cast `/Game/FPS_Game/Blueprints/BP_CharacterBase` OtherActor))
  (`Widget.SetVisibility` (`/Game/FPS_Game/UI/W_PlayerHUD.InteractPrompt_TXT` (`/Game/FPS_Game/Blueprints/BP_CharacterBase.PlayerHUD` _asbp_character_base)) "Visible")
  (`PrimitiveComponent.SetRenderCustomDepth` (`self.Top`) true)
  (`PrimitiveComponent.SetRenderCustomDepth` (`self.Bottom`) true)
  (`PrimitiveComponent.SetRenderCustomDepth` (`self.SideL`) true)
  (`PrimitiveComponent.SetRenderCustomDepth` (`self.SideR`) true)
  (`PrimitiveComponent.SetRenderCustomDepth` (`self.SideF`) true)
  (`PrimitiveComponent.SetRenderCustomDepth` (`self.SideB`) true))

(event `self.ReceiveActorEndOverlap`
  (params (OtherActor :type "Actor Object Reference"))
  (bind _asbp_character_base (cast `/Game/FPS_Game/Blueprints/BP_CharacterBase` OtherActor))
  (`Widget.SetVisibility` (`/Game/FPS_Game/UI/W_PlayerHUD.InteractPrompt_TXT` (`/Game/FPS_Game/Blueprints/BP_CharacterBase.PlayerHUD` _asbp_character_base)) "Hidden")
  (`PrimitiveComponent.SetRenderCustomDepth` (`self.Top`) false)
  (`PrimitiveComponent.SetRenderCustomDepth` (`self.Bottom`) false)
  (`PrimitiveComponent.SetRenderCustomDepth` (`self.SideL`) false)
  (`PrimitiveComponent.SetRenderCustomDepth` (`self.SideF`) false)
  (`PrimitiveComponent.SetRenderCustomDepth` (`self.SideB`) false)
  (`PrimitiveComponent.SetRenderCustomDepth` (`self.SideR`) false))

(event `/Game/FPS_Game/Blueprints/System/BPI_Interact.BPI_Interaction`
  (`/Engine/EditorBlueprintResources/StandardMacros.DoOnce` false
    (:`Completed`
      (`GameplayStatics.SpawnSoundAtLocation` "/Game/FPS_Game/Sounds/SFX/Weapon_AssaultRifle/Mono/AssaultRifle_Equip_Cue.AssaultRifle_Equip_Cue" (`self.K2_GetActorLocation`))
      (bind (_direction _alpha) (`Timeline|OpenDoor` :!via `PlayFromStart`)
        (:`Update`
          (`SceneComponent.K2_SetRelativeRotation` (`self.Top`) (`KismetMathLibrary.RLerp` (struct) (struct :`Roll` 45.0) _alpha) false false)
          (`PrimitiveComponent.SetCollisionEnabled` (`self.Box`) "NoCollision"))
        (:`Finished`
          (`/Engine/EditorBlueprintResources/StandardMacros.DoOnce` false
            (:`Completed`
              (`self.SpawnLoot`))))))))

(event `SpawnLoot`
  (bind _sphere1 (`self.Sphere1`))
  (bind _sphere (`self.Sphere`))
  (`|ExecutionSequence`
    (:`then_0`
      (`self.RandomSwitchOnIntAndSpawn` (`SceneComponent.K2_GetComponentLocation` _sphere) (`SceneComponent.K2_GetComponentRotation` _sphere)))
    (:`then_1`
      (`self.RandomSwitchOnIntAndSpawn` (`SceneComponent.K2_GetComponentLocation` _sphere1) (`SceneComponent.K2_GetComponentRotation` _sphere1)))))

(fn `RandomSwitchOnIntAndSpawn`
  (params (`Spawn Transform Location` :type "Vector Structure") (`Spawn Transform Rotation` :type "Rotator Structure"))
  (switch `int` (`KismetMathLibrary.RandomIntegerInRange` 0 7)
    (:`0`
      (`|SpawnActorFromClass` "/Game/FPS_Game/Blueprints/Weapons/BPC_WeaponLaser.BPC_WeaponLaser_C" (`KismetMathLibrary.MakeTransform` `Spawn Transform Location` `Spawn Transform Rotation` (1.0 1.0 1.0)) "AlwaysSpawn" "OverrideRootScale" null null))
    (:`1`
      (`|SpawnActorFromClass` "/Game/FPS_Game/Blueprints/Weapons/BPC_WeaponLauncher.BPC_WeaponLauncher_C" (`KismetMathLibrary.MakeTransform` `Spawn Transform Location` `Spawn Transform Rotation`) "AlwaysSpawn" "OverrideRootScale" null null))
    (:`2`
      (`|SpawnActorFromClass` "/Game/FPS_Game/Blueprints/Weapons/BPC_WeaponPistol.BPC_WeaponPistol_C" (`KismetMathLibrary.MakeTransform` `Spawn Transform Location` `Spawn Transform Rotation`) "AlwaysSpawn" "OverrideRootScale" null null))
    (:`3`
      (`|SpawnActorFromClass` "/Game/FPS_Game/Blueprints/Weapons/BPC_WeaponPistolAuto.BPC_WeaponPistolAuto_C" (`KismetMathLibrary.MakeTransform` `Spawn Transform Location` `Spawn Transform Rotation`) "AlwaysSpawn" "OverrideRootScale" null null))
    (:`4`
      (`|SpawnActorFromClass` "/Game/FPS_Game/Blueprints/Weapons/BPC_WeaponRecoil.BPC_WeaponRecoil_C" (`KismetMathLibrary.MakeTransform` `Spawn Transform Location` `Spawn Transform Rotation`) "AlwaysSpawn" "OverrideRootScale" null null))
    (:`5`
      (`|SpawnActorFromClass` "/Game/FPS_Game/Blueprints/Weapons/BPC_WeaponRifle.BPC_WeaponRifle_C" (`KismetMathLibrary.MakeTransform` `Spawn Transform Location` `Spawn Transform Rotation`) "AlwaysSpawn" "OverrideRootScale" null null))
    (:`6`
      (`|SpawnActorFromClass` "/Game/FPS_Game/Blueprints/Weapons/BPC_WeaponShotgun.BPC_WeaponShotgun_C" (`KismetMathLibrary.MakeTransform` `Spawn Transform Location` `Spawn Transform Rotation`) "AlwaysSpawn" "OverrideRootScale" null null))
    (:`7`
      (`|SpawnActorFromClass` "/Game/FPS_Game/Blueprints/Weapons/BPC_WeaponSniper.BPC_WeaponSniper_C" (`KismetMathLibrary.MakeTransform` `Spawn Transform Location` `Spawn Transform Rotation`) "AlwaysSpawn" "OverrideRootScale" null null))))

(fn `UserConstructionScript`)